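; Trigger box that tells the first-person character when it is within range, through its IsInRangeE flag.
; On begin overlap it casts the actor to FirstPersonCharacter, stores it as Player and sets the flag.
; On end overlap it clears the flag if the leaving actor is that stored Player.
; Tick prints a constant false every frame, independent of the overlap state.
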(event `self.ReceiveTick`
  (params (DeltaSeconds :type "Float (single-precision)"))
  (`KismetSystemLibrary.PrintString` (`KismetStringLibrary.Conv_BoolToString` false)))

(event `Key|E`
  (params (Key :type "Key Structure")))

(event `self.ReceiveActorBeginOverlap`
  (params (OtherActor :type "Actor Object Reference"))
  (bind _asfirst_person_character (cast `/Game/FirstPersonBP/Blueprints/FirstPersonCharacter` OtherActor))
  (bind _output_get (set `self.Player` _asfirst_person_character))
  (set `/Game/FirstPersonBP/Blueprints/FirstPersonCharacter.isInRangeE` true _output_get))

(event `self.ReceiveActorEndOverlap`
  (params (OtherActor :type "Actor Object Reference"))
  (bind _player (`self.Player`))
  (if (== OtherActor _player)
    (set `/Game/FirstPersonBP/Blueprints/FirstPersonCharacter.isInRangeE` false _player)))

(fn `UserConstructionScript`)