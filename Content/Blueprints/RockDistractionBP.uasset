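; RockDistractionBP is a rock decoy that makes noise where it lands.
; Its first hit on anything but the player writes the Sphere's position to the PC_Proje parameter collection and starts a timeline animating its Radius.
; Each timeline update also plays the rock sound, reports a DecoyTag noise event instigated by the player, and resets a short actor lifespan.
; Radius returns to zero when the timeline finishes.
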(event `self.ReceiveHit`
  (params (MyComp :type "PrimitiveComponent Object Reference") (Other :type "Actor Object Reference") (OtherComp :type "PrimitiveComponent Object Reference") (bSelfMoved :type Boolean) (HitLocation :type "Vector Structure") (HitNormal :type "Vector Structure") (NormalImpulse :type "Vector Structure") (Hit :type "HitResult Structure (by ref)"))
  (bind _returnvalue (`GameplayStatics.GetPlayerCharacter` 0))
  (bind _returnvalue_2 (`self.K2_GetActorLocation`))
  (if (!= Other _returnvalue)
    (`/Engine/EditorBlueprintResources/StandardMacros.DoOnce` false
      (:`Completed`
        (`KismetSystemLibrary.PrintString` "Hello")
        (`KismetMaterialLibrary.SetVectorParameterValue` "/Game/FirstPersonBP/Materials/PC_Proje.PC_Proje" "Position" (`KismetMathLibrary.Conv_VectorToLinearColor` (`SceneComponent.K2_GetComponentLocation` (`self.Sphere`))))
        (bind (_direction _newtrack_0) (`Timeline|Timeline_0` :!via `PlayFromStart`)
          (:`Update`
            (`KismetMaterialLibrary.SetScalarParameterValue` "/Game/FirstPersonBP/Materials/PC_Proje.PC_Proje" "Radius" _newtrack_0)
            (`GameplayStatics.PlaySoundAtLocation` "/Game/Sound/RockAudioCue.RockAudioCue" _returnvalue_2 (struct) 1.0 1.0 0.0 null null null)
            (`AISense_Hearing.ReportNoiseEvent` _returnvalue_2 1.0 _returnvalue 1000.0 (`self.DecoyTag`))
            (`self.SetLifeSpan` 0.2))
          (:`Finished`
            (`KismetMaterialLibrary.SetScalarParameterValue` "/Game/FirstPersonBP/Materials/PC_Proje.PC_Proje" "Radius")))))))

(fn `UserConstructionScript`)