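; Coin distraction decoy that broadcasts an expanding radius effect from where its Piece first hits something other than the player.
; That impact writes the location to the PC_Proje material parameter collection and starts a timeline driving Radius.
; Once Radius reaches 1, a second timeline drives Rad, then zeroes both on finish.
; Every hit also sets the actor's lifespan, and construction sets its Decoy tag variable.
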(event `self.Piece.OnComponentHit`
  (params (HitComponent :type "PrimitiveComponent Object Reference") (OtherActor :type "Actor Object Reference") (OtherComp :type "PrimitiveComponent Object Reference") (NormalImpulse :type "Vector Structure") (Hit :type "HitResult Structure (by ref)"))
  (`|ExecutionSequence`
    (:`then_0`
      (if (!= OtherActor (`GameplayStatics.GetPlayerCharacter` 0))
        (`/Engine/EditorBlueprintResources/StandardMacros.DoOnce` false
          (:`Completed`
            (`KismetMaterialLibrary.SetVectorParameterValue` "/Game/FirstPersonBP/Materials/PC_Proje.PC_Proje" "Position" (`KismetMathLibrary.Conv_VectorToLinearColor` (`SceneComponent.K2_GetComponentLocation` (`self.Piece`))))
            (bind (_direction _newtrack_0) (`Timeline|Timeline_0` :!via `PlayFromStart`)
              (:`Update`
                (`KismetMaterialLibrary.SetScalarParameterValue` "/Game/FirstPersonBP/Materials/PC_Proje.PC_Proje" "Radius" _newtrack_0)
                (bind _returnvalue (`KismetMaterialLibrary.GetScalarParameterValue` "/Game/FirstPersonBP/Materials/PC_Proje.PC_Proje" "Radius"))
                (if (>= _returnvalue 1.0)
                  (bind (_direction_2 _newtrack_0_2) (`Timeline|Timeline_1` :!via `PlayFromStart`)
                    (:`Update`
                      (`KismetMaterialLibrary.SetScalarParameterValue` "/Game/FirstPersonBP/Materials/PC_Proje.PC_Proje" "Rad" _newtrack_0_2))
                    (:`Finished`
                      (`KismetMaterialLibrary.SetScalarParameterValue` "/Game/FirstPersonBP/Materials/PC_Proje.PC_Proje" "Rad")
                      (`KismetMaterialLibrary.SetScalarParameterValue` "/Game/FirstPersonBP/Materials/PC_Proje.PC_Proje" "Radius"))))))))))
    (:`then_1`
      (`self.SetLifeSpan` (`self.LifespanDecoy`)))))

(fn `UserConstructionScript`
  (set `self.DecoyTag` "Decoy") ; just in case
)