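; Map sign actor that lets the first-person player interact with a map when standing inside its trigger box.
; On overlap it stores the player, sets their IsInRangeE flag and registers itself as their MapInteraction target.
; When that player leaves, it clears the flag and removes top-level Widget_Map widgets from the screen.
; Opening the map is not handled in this Blueprint.
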(event `self.Box.OnComponentBeginOverlap`
  (params (OverlappedComponent :type "PrimitiveComponent Object Reference") (OtherActor :type "Actor Object Reference") (OtherComp :type "PrimitiveComponent Object Reference") (OtherBodyIndex :type Integer) (bFromSweep :type Boolean) (SweepResult :type "HitResult Structure (by ref)"))
  (bind _asfirst_person_character (cast `/Game/FirstPersonBP/Blueprints/FirstPersonCharacter` OtherActor))
  (bind _output_get (set `self.Player` _asfirst_person_character))
  (set `/Game/FirstPersonBP/Blueprints/FirstPersonCharacter.isInRangeE` true _output_get)
  (set `/Game/FirstPersonBP/Blueprints/FirstPersonCharacter.Map Interaction` self _asfirst_person_character))

(event `self.Box.OnComponentEndOverlap`
  (params (OverlappedComponent :type "PrimitiveComponent Object Reference") (OtherActor :type "Actor Object Reference") (OtherComp :type "PrimitiveComponent Object Reference") (OtherBodyIndex :type Integer))
  (bind _player (`self.Player`))
  (if (== OtherActor _player)
    (set `/Game/FirstPersonBP/Blueprints/FirstPersonCharacter.isInRangeE` false _player)
    (bind _foundwidgets (`WidgetBlueprintLibrary.GetAllWidgetsOfClass` "/Game/Blueprints/UI/Widget_Map.Widget_Map_C"))
    (`Widget.RemoveFromParent` _foundwidgets)))

(fn `UserConstructionScript`)