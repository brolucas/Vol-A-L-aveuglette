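; Actor component that plays an impact sound and reports an AI noise event when its owner hits something.
; It binds to the owner's OnActorHit and spawns the sound at the hit location.
; The owner's velocity is remapped to drive the sound's "power" parameter and volume, plus the noise's loudness and range.
; A DoOnce reset after a short random delay throttles repeated hits.
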(event `self.ReceiveBeginPlay`
  (add `Actor.OnActorHit` (`self.GetOwner`) (delegate `HitGround`)) ; Abonne l'owner a l'event On Hit
)

(event `HitGround`
  (params (SelfActor :type "Actor Object Reference") (OtherActor :type "Actor Object Reference") (NormalImpulse :type "Vector Structure") (Hit :type "HitResult Structure (by ref)"))
  (bind _returnvalue (`KismetMathLibrary.VSize` (`Actor.GetVelocity` SelfActor)))
  (bind _returnvalue_2 (`KismetMathLibrary.MapRangeClamped` _returnvalue 30.0 0.0 1.0))
  (bind _returnvalue_3 (`KismetMathLibrary.MapRangeClamped` _returnvalue 400.0 30.0 0.0 5.0))
  (`|ExecutionSequence`
    (:`then_0`
      (`/Engine/EditorBlueprintResources/StandardMacros.DoOnce` false :!label _label
        (:`Completed`
          (bind _returnvalue_4 (`GameplayStatics.SpawnSoundAtLocation` (`self.Sound`) (`.Location` (`GameplayStatics.BreakHitResult` Hit)) (struct) 1.0 1.0 0.0 null null))
          (`AudioComponent.SetIntParameter` _returnvalue_4 "power" (`KismetMathLibrary.FTrunc` _returnvalue_3))
          (`AudioComponent.SetVolumeMultiplier` _returnvalue_4 _returnvalue_2)
          (`AISense_Hearing.ReportNoiseEvent` (0.0 0.0 0.0) _returnvalue_2 null _returnvalue_3))))
    (:`then_1`
      (`KismetSystemLibrary.Delay` (`KismetMathLibrary.RandomFloatInRange` 0.1 0.2))
      (goto _label :!via `Reset`))))